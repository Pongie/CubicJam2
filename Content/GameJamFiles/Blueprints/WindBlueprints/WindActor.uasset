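; WindActor is a moving wind gust that affects the player's ship on contact.
; On BeginPlay it writes DestinationVector into its InterpToMovement as an absolute control point, then destroys itself when that movement stops.
; The first ShipPawn overlapping its Box gets its turn cooldown set, its delay retriggered and its wind collision speed trigger called.
; Random destination picking from WindSpawner boxes is left disconnected, and GenerateDestination is empty.
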(event `self.ReceiveBeginPlay`
  (`KismetArrayLibrary.Array_Set` (`InterpToMovementComponent.ControlPoints` (`self.InterpToMovement`)) 1 (make `InterpControlPoint` (`self.DestinationVector`) false)))

(event `GenerateDestination`)

(event `self.InterpToMovement.OnResetDelegate`
  (params (ImpactResult :type "HitResult Structure (by ref)") (Time :type "Float (single-precision)")))

(event `self.InterpToMovement.OnInterpToStop`
  (params (ImpactResult :type "HitResult Structure (by ref)") (Time :type "Float (single-precision)"))
  (`self.K2_DestroyActor`))

(event `self.Box.OnComponentBeginOverlap`
  (params (OverlappedComponent :type "PrimitiveComponent Object Reference") (OtherActor :type "Actor Object Reference") (OtherComp :type "PrimitiveComponent Object Reference") (OtherBodyIndex :type Integer) (bFromSweep :type Boolean) (SweepResult :type "HitResult Structure (by ref)"))
  (bind _asship_pawn (cast `/Game/GameJamFiles/Blueprints/ShipPawn` OtherActor))
  (`/Engine/EditorBlueprintResources/StandardMacros.DoOnce` false
    (:`Completed`
      (set `/Game/GameJamFiles/Blueprints/ShipPawn.TurnCooldown` 1.0 _asship_pawn)
      (`/Game/GameJamFiles/Blueprints/ShipPawn.RetriggerDelay` _asship_pawn)
      (`/Game/GameJamFiles/Blueprints/ShipPawn.WindCollisionSpeedTrigger` _asship_pawn))))

(fn `UserConstructionScript`)