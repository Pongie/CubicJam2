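; WindSpawner periodically spawns scaled-up WindActors that are each given a destination inside a spawner's box.
; After a startup delay, it reads the spawner array from CustomGameMode and starts a looping timer with a randomized interval chosen once.
; Each tick compares itself to a random entry's Box, retrying on a match, then re-rolls the destination.
; Start and destination are random points within the two boxes.
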(event `self.ReceiveBeginPlay`
  ;[0.8373 0.4339 1] MAGIC!
  (`KismetSystemLibrary.Delay` 2.0)
  (bind _ascustom_game_mode (cast `/Game/GameJamFiles/Blueprints/CustomGameMode` (`GameplayStatics.GetGameMode`))
    (:`then`
      (set `self.ArrayOfSpawners` (`/Game/GameJamFiles/Blueprints/CustomGameMode.ArrayOfSpawners` _ascustom_game_mode))
      (`KismetSystemLibrary.K2_SetTimerDelegate` (delegate `GenerateDestination`) (`KismetMathLibrary.RandomFloatInRange` 2.0 4.0) true))
    (:`CastFailed`
      (`KismetSystemLibrary.PrintString` "Cast To Game Mode Failed In WindSpawner"))))

(event `GenerateDestination`
  (bind _box (`self.Box`))
  (bind _arrayofspawners (`self.ArrayOfSpawners`))
  (bind _destinationspawner (`self.DestinationSpawner`))
  (bind _box_2 (`/Game/GameJamFiles/Blueprints/WindBlueprints/WindSpawner.Box` (`|GetArrayItem` _arrayofspawners (`KismetMathLibrary.RandomIntegerInRange` 0 (- (`KismetArrayLibrary.Array_Length` _arrayofspawners) 1)))))
  (if (== self _box_2) :!label _label
    (`KismetSystemLibrary.Delay` 0.1)
    (goto _label)
    (else
      (bind _output_get (set `self.DestinationSpawner` _box_2))
      (`|SpawnActorFromClass` "/Game/GameJamFiles/Blueprints/WindBlueprints/WindActor.WindActor_C" (`KismetMathLibrary.MakeTransform` (`KismetMathLibrary.RandomPointInBoundingBox` (`SceneComponent.K2_GetComponentLocation` _box) (`BoxComponent.GetScaledBoxExtent` _box)) (struct) (10.0 10.0 10.0)) "Undefined" "OverrideRootScale" null (`KismetMathLibrary.RandomPointInBoundingBox` (`SceneComponent.K2_GetComponentLocation` _destinationspawner) (`BoxComponent.GetScaledBoxExtent` _destinationspawner)) null))))

(fn `UserConstructionScript`)