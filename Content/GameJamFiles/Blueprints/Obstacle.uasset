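; Rock obstacle for the ship game that picks a random small, medium or large mesh from its size setting.
; The construction script sizes the collision sphere to match, applies a slight random rotation and pins the actor to a fixed Z height.
; Sphere hits are checked on authority against the ship pawn's Box and only print a debug message.
; SetupCollision and the unfinished ConstructIsland are uncalled legacy functions.
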(event `self.CollisionSphere.OnComponentHit`
  (params (HitComponent :type "PrimitiveComponent Object Reference") (OtherActor :type "Actor Object Reference") (OtherComp :type "PrimitiveComponent Object Reference") (NormalImpulse :type "Vector Structure") (Hit :type "HitResult Structure (by ref)"))
  (`/Engine/EditorBlueprintResources/ActorMacros.Switch Has Authority`
    (:`Authority`
      (bind _asship_pawn (cast `/Game/GameJamFiles/Blueprints/ShipPawn` OtherActor))
      (if (== (`/Game/GameJamFiles/Blueprints/ShipPawn.Box` _asship_pawn) (`.HitComponent` (`GameplayStatics.BreakHitResult` Hit)))
        (`KismetSystemLibrary.PrintString` "Hit the Rocks!" true true (struct :`R` 1.0 :`G` 0.029323 :`A` 1.0) 3.0)))))

(fn `Construct Island`
  (locals (IslandPiece :type Integer) (IslandPiece2 :type Integer) (PotIsland3 :type Integer) (PotIsland4 :type Integer) (PotIsland5 :type Integer) (PotIsland6 :type Integer) (NoMoreAdditionalIslands :type Boolean) (BonusIslandstoGenerate :type Integer) (IslandCounter :type Integer :default 1) (AdditionalIslands :type "Array of Integer") (AdjustmentVector :type "Vector Structure") (AdjustmentTransform :type "Transform Structure"))
  (bind _islandcounter (`local.IslandCounter`))
  (bind _additionalislands (`local.AdditionalIslands`))
  ;[1 1 1] Determine Pieces
  ;;[1 1 1] Legacy - Time sink
  (set `local.IslandPiece` (`KismetMathLibrary.RandomIntegerInRange` 0 5))
  (set `local.IslandPiece2` (`KismetMathLibrary.RandomIntegerInRange` 0 5))
  (if (>= (`KismetMathLibrary.RandomFloatInRange` 0.0 100.0) 66.699997)
    (bind _output_get (set `local.BonusIslandstoGenerate` (`KismetMathLibrary.RandomIntegerInRange` 0 4)))
    (if (>= _output_get 0)
      (while (`local.NoMoreAdditionalIslands`)
        (`KismetArrayLibrary.Array_Add` _additionalislands (`KismetMathLibrary.RandomIntegerInRange` 0 5))
        (`/Engine/EditorBlueprintResources/StandardMacros.IncrementInt` _islandcounter
          (:`  `
            (set `local.NoMoreAdditionalIslands` (== _islandcounter (`local.BonusIslandstoGenerate`))))))
      (for (_array_element _array_index) _additionalislands
        (switch `int` _array_index
          (:`0`
            (set `local.PotIsland3` _array_element))
          (:`1`
            (set `local.PotIsland4` _array_element))
          (:`2`
            (set `local.PotIsland5` _array_element))
          (:`3`
            (set `local.PotIsland6` _array_element))))))
  ;[1 1 1] Offset Location
  (for _array_element_2 (`|MakeArray` (`self.Mesh`) (`self.Mesh2`) (`self.Mesh3`) (`self.Mesh4`) (`self.Mesh5`) (`self.Mesh6`))
    (if (!= _array_element_2 null)
      (switch `int` (`KismetMathLibrary.RandomIntegerInRange` 0 1))
      (else
        (break)))))

(fn `Setup Collision`
  (params (ObstacleID :type Integer) (ChosenMesh :type Integer))
  (locals (LocalCollisionSize :type "Transform Structure"))
  (bind _smeshesarray (`self.SMeshesArray`))
  (bind _mmeshesarray (`self.MMeshesArray`))
  (bind _lmeshesarray (`self.LMeshesArray`))
  (bind _collisionsphere (`self.CollisionSphere`))
  ;[1 1 1] Legacy Function - No need for 2
  (`|ExecutionSequence`
    (:`then_0`)
    (:`then_1`
      (switch `int` ObstacleID
        (:`0`
          (`StaticMeshComponent.SetStaticMesh` (`self.Mesh`) (`|GetArrayItem` _smeshesarray (`KismetMathLibrary.RandomIntegerInRange` 0 (- (`KismetArrayLibrary.Array_Length` _smeshesarray) 1))))
          (`SphereComponent.SetSphereRadius` _collisionsphere 100.0 true))
        (:`1`
          (`StaticMeshComponent.SetStaticMesh` (`self.Mesh`) (`|GetArrayItem` _mmeshesarray (`KismetMathLibrary.RandomIntegerInRange` 0 (- (`KismetArrayLibrary.Array_Length` _mmeshesarray) 1))))
          (`SphereComponent.SetSphereRadius` _collisionsphere 500.0 true))
        (:`2`
          (`StaticMeshComponent.SetStaticMesh` (`self.Mesh`) (`|GetArrayItem` _lmeshesarray (`KismetMathLibrary.RandomIntegerInRange` 0 (- (`KismetArrayLibrary.Array_Length` _lmeshesarray) 1))))
          (`SphereComponent.SetSphereRadius` _collisionsphere 2500.0 true))))))

(fn `Setup Mesh`
  (params (ObstacleID :type Integer))
  (bind _smeshesarray (`self.SMeshesArray`))
  (bind _mmeshesarray (`self.MMeshesArray`))
  (bind _lmeshesarray (`self.LMeshesArray`))
  (bind _collisionsphere (`self.CollisionSphere`))
  (switch `int` ObstacleID
    (:`0`
      (`StaticMeshComponent.SetStaticMesh` (`self.Mesh`) (`|GetArrayItem` _smeshesarray (`KismetMathLibrary.RandomIntegerInRange` 0 (- (`KismetArrayLibrary.Array_Length` _smeshesarray) 1))))
      (`SphereComponent.SetSphereRadius` _collisionsphere 150.0 true))
    (:`1`
      (`StaticMeshComponent.SetStaticMesh` (`self.Mesh`) (`|GetArrayItem` _mmeshesarray (`KismetMathLibrary.RandomIntegerInRange` 0 (- (`KismetArrayLibrary.Array_Length` _mmeshesarray) 1))))
      (`SphereComponent.SetSphereRadius` _collisionsphere 500.0 true))
    (:`2`
      (set `self.ChosenMesh` 0)
      (`StaticMeshComponent.SetStaticMesh` (`self.Mesh`) (`|GetArrayItem` _lmeshesarray (`KismetMathLibrary.RandomIntegerInRange` 0 (- (`KismetArrayLibrary.Array_Length` _lmeshesarray) 1))))
      (`SphereComponent.SetSphereRadius` _collisionsphere 1600.0 true))
    (:`3`)))

(fn `UserConstructionScript`
  (`self.Setup Mesh` (`self.ObstacleSize`))
  (`SceneComponent.K2_SetWorldRotation` (`self.Mesh`) (`KismetMathLibrary.MakeRotator` (`KismetMathLibrary.FClamp` (`KismetMathLibrary.RandomFloat`) -32.0 32.0) (`KismetMathLibrary.FClamp` (`KismetMathLibrary.RandomFloat`) -32.0 32.0) (`KismetMathLibrary.FClamp` (`KismetMathLibrary.RandomFloat`) -32.0 32.0)) false false)
  ;[1 1 1] Always Root Z plane
  (`self.K2_SetActorLocation` (`KismetMathLibrary.MakeVector` (.x (`self.K2_GetActorLocation`)) (.y (`self.K2_GetActorLocation`)) 133.0)))